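; Prototype shield Blueprint that acts as a destructible barrier with its own Health.
; Each Hit event subtracts a fixed amount of Health, and Tick clears IsActive once Health is depleted.
; Every Tick also applies IsActive to the components, making the Sphere block all channels and showing the Shield while active, or ignoring collision and hiding it otherwise.
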(event EventBeginPlay)

(event Collision|EventActorBeginOverlap
  (params (OtherActor :type Actor%20Object%20Reference)))

(event EventTick
  (params (DeltaSeconds :type Float%20%28single-precision%29))
  (Utilities|FlowControl|Sequence
    (:then_0
      (if (<= (Variables|Default|GetHealth) 0.0)
        (Variables|Default|SetIsActive false)))
    (:then_1
      (if (Variables|Default|GetIsActive)
        (Collision|SetCollisionResponsetoAllChannels (Variables|Default|GetSphere) "ECR_Block")
        (Rendering|SetVisibility (Variables|Default|Getshield) true true)
        (else
          (Collision|SetCollisionResponsetoAllChannels (Variables|Default|GetSphere) "ECR_Ignore")
          (Rendering|SetVisibility (Variables|Default|Getshield) false true))))))

(event Collision|EventHit
  (params (MyComp :type Primitive%20Component%20Object%20Reference) (Other :type Actor%20Object%20Reference) (OtherComp :type Primitive%20Component%20Object%20Reference) (bSelfMoved :type Boolean) (HitLocation :type Vector :default "0, 0, 0") (HitNormal :type Vector :default "0, 0, 0") (NormalImpulse :type Vector :default "0, 0, 0") (Hit :type Hit%20Result%20Structure%20%28by%20ref%29))
  (Variables|Default|SetHealth (- (Variables|Default|GetHealth) 1e+01)))

(fn ConstructionScript)