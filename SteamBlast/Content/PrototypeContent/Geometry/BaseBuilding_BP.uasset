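; Base building prototype Blueprint with four spots where a VR character carrying a device can reveal a mesh by entering a trigger box.
; On BeginPlay it spawns four Goal actors and attaches each to its own scene component.
; Each box overlap passes its paired mesh through a server event to a multicast event, which makes it visible if the VR_Character3 has a device.
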(event OnComponentBeginOverlap(Box3)
  (params (OverlappedComponent :type Primitive%20Component%20Object%20Reference) (OtherActor :type Actor%20Object%20Reference) (OtherComp :type Primitive%20Component%20Object%20Reference) (OtherBodyIndex :type Integer) (bFromSweep :type Boolean) (SweepResult :type Hit%20Result%20Structure%20%28by%20ref%29))
  (CallFunction|ActivateDeviceonServer OtherActor (Variables|Default|GetStaticMesh3)))

(event OnComponentBeginOverlap(Box2)
  (params (OverlappedComponent :type Primitive%20Component%20Object%20Reference) (OtherActor :type Actor%20Object%20Reference) (OtherComp :type Primitive%20Component%20Object%20Reference) (OtherBodyIndex :type Integer) (bFromSweep :type Boolean) (SweepResult :type Hit%20Result%20Structure%20%28by%20ref%29))
  (CallFunction|ActivateDeviceonServer OtherActor (Variables|Default|GetStaticMesh2)))

(event OnComponentBeginOverlap(Box1)
  (params (OverlappedComponent :type Primitive%20Component%20Object%20Reference) (OtherActor :type Actor%20Object%20Reference) (OtherComp :type Primitive%20Component%20Object%20Reference) (OtherBodyIndex :type Integer) (bFromSweep :type Boolean) (SweepResult :type Hit%20Result%20Structure%20%28by%20ref%29))
  (CallFunction|ActivateDeviceonServer OtherActor (Variables|Default|GetStaticMesh1)))

(event OnComponentBeginOverlap(Box)
  (params (OverlappedComponent :type Primitive%20Component%20Object%20Reference) (OtherActor :type Actor%20Object%20Reference) (OtherComp :type Primitive%20Component%20Object%20Reference) (OtherBodyIndex :type Integer) (bFromSweep :type Boolean) (SweepResult :type Hit%20Result%20Structure%20%28by%20ref%29))
  (CallFunction|ActivateDeviceonServer OtherActor (Variables|Default|GetStaticMesh)))

(event Custom|ActivateDeviceMulticast
  (params (Actor :type Actor%20Object%20Reference) (Mesh :type Static%20Mesh%20Component%20Object%20Reference))
  (bind _asvr_character_3 (Utilities|Casting|CastToVR_Character3 Actor))
  (if (Variables|/Game/PrototypeContent/Players/VR_Character3.VR_Character3_C|GetHasDevice _asvr_character_3)
    (Rendering|SetVisibility Mesh true false)))

(event Custom|ActivateDeviceOnServer
  (params (Actor :type Actor%20Object%20Reference) (Mesh :type Static%20Mesh%20Component%20Object%20Reference))
  (CallFunction|ActivateDeviceMulticast Actor Mesh))

(event EventBeginPlay
  (Utilities|FlowControl|Sequence
    (:then_0
      (bind _returnvalue (Game|SpawnActorfromClass "/Game/PrototypeContent/Goal.Goal_C" (Transformation|GetWorldTransform (Variables|Default|GetScene)) "Undefined" 0 0))
      (Transformation|AttachComponentToComponent _returnvalue (Variables|Default|GetScene) "None" "KeepWorld" "KeepRelative" "KeepRelative" true))
    (:then_1
      (bind _returnvalue_2 (Game|SpawnActorfromClass "/Game/PrototypeContent/Goal.Goal_C" (Transformation|GetWorldTransform (Variables|Default|GetScene1)) "Undefined" 0 0))
      (Transformation|AttachComponentToComponent _returnvalue_2 (Variables|Default|GetScene1) "None" "KeepWorld" "KeepRelative" "KeepRelative" true))
    (:then_2
      (bind _returnvalue_3 (Game|SpawnActorfromClass "/Game/PrototypeContent/Goal.Goal_C" (Transformation|GetWorldTransform (Variables|Default|GetScene2)) "Undefined" 0 0))
      (Transformation|AttachComponentToComponent _returnvalue_3 (Variables|Default|GetScene2) "None" "KeepWorld" "KeepRelative" "KeepRelative" true))
    (:then_3
      (bind _returnvalue_4 (Game|SpawnActorfromClass "/Game/PrototypeContent/Goal.Goal_C" (Transformation|GetWorldTransform (Variables|Default|GetScene3)) "Undefined" 0 0))
      (Transformation|AttachComponentToComponent _returnvalue_4 (Variables|Default|GetScene3) "None" "KeepWorld" "KeepRelative" "KeepRelative" true))))

(event Collision|EventActorBeginOverlap
  (params (OtherActor :type Actor%20Object%20Reference)))

(event EventTick
  (params (DeltaSeconds :type Float%20%28single-precision%29)))

(fn ConstructionScript)